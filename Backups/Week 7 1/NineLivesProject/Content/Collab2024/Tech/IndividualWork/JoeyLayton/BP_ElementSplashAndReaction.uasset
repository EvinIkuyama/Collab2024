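; Short-lived elemental splash area that combines with overlapping reactive actors to trigger effects based on Fire, Wind, Water and Earth pairings.
; BeginPlay adds an AOE box and Niagara effect; on overlap, the older BPI_Reactive actor resolves the order-independent reaction and destroys both.
; Reactions apply blast impulses, spawn platforms or rocks, or spawn non-stacking player buff actors via sphere queries.
; Fire explosion, obsidian/meteorite, water bubble and sticky surface are print-only stubs.
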(event Custom|OnReact_Blast
  ;[1 0.3534 0.3833] Explosion
  (Development|PrintString "Blast")
  (Niagara|SpawnSystematLocation "/Game/Collab2024/Tech/IndividualWork/JoeyLayton/NiagaraEffects/PS_Reaction_Burst.PS_Reaction_Burst" (Transformation|GetActorLocation))
  (bind (_out_actors _player_ref) (CallFunction|GetMoveableinArea))
  ;;[1 1 1] Player Impulse
  (bind _asbp_main_character (Utilities|Casting|CastToBP_MainCharacter _player_ref)
    (:then
      (Physics|AddImpulse (Variables|/Script/Engine.Character|GetCharacterMovement _asbp_main_character) (Math|Vector|MakeVector (.X (Math|Vector|BreakVector (Transformation|GetVelocity _player_ref))) (.Y (Math|Vector|BreakVector (Transformation|GetVelocity _player_ref))) 1e+05) false))
    (:CastFailed
      _))
  ;;[1 1 1] Enemy Impulse
  (for _array_element _out_actors
    (Physics|AddImpulse (Actor|GetComponentbyClass _array_element "/Script/Engine.PrimitiveComponent") (Math|Vector|MakeVector (* 1e+03 (.X (Math|Vector|BreakVector (- (Transformation|GetActorLocation _array_element) (Transformation|GetActorLocation))))) (* (.Y (Math|Vector|BreakVector (- (Transformation|GetActorLocation _array_element) (Transformation|GetActorLocation)))) 1e+03) 5e+04) "None" false)))

(event Custom|OnReact_SpeedBoost
  ;[0.6926 0.6739 1] Speed Boost
  (Development|PrintString "Speed Boost")
  ;;[1 1 1] Ensures speed can't be stacked
  (bind _outactors (Actor|GetAllActorsOfClass "/Game/Collab2024/Tech/IndividualWork/JoeyLayton/Reactions/BP_PlayerReaction_SpeedBoost.BP_PlayerReaction_SpeedBoost_C"))
  (if (Utilities|Array|IsEmpty _outactors)
    (bind _output_get (CallFunction|GetPlayerinArea))
    ;;[1 1 1] Spawns speed boost actor
    (bind _asbp_main_character (Utilities|Casting|CastToBP_MainCharacter _output_get))
    (Game|SpawnActorfromClass "/Game/Collab2024/Tech/IndividualWork/JoeyLayton/Reactions/BP_PlayerReaction_SpeedBoost.BP_PlayerReaction_SpeedBoost_C" (Math|Conversions|ToTransform(Vector) "0, 0, 0") "Undefined" "MultiplyWithRoot" 0 _asbp_main_character 0)))

(event Custom|OnReact_ObsidianOrMeteorite
  (Development|PrintString "Obsidian or Meteorite"))

(event Custom|OnReact_DoubleJump
  ;[1 0.3036 0.7057] Double Jump
  (Development|PrintString "Double Jump")
  ;;[1 1 1] Ensures double jumps can't be stacked
  (bind _outactors (Actor|GetAllActorsOfClass "/Game/Collab2024/Tech/IndividualWork/JoeyLayton/Reactions/BP_PlayerReaction_DoubleJump.BP_PlayerReaction_DoubleJump_C"))
  (if (Utilities|Array|IsEmpty _outactors)
    (bind _output_get (CallFunction|GetPlayerinArea))
    ;;[1 1 1] Spawns double jump actor
    (bind _asbp_main_character (Utilities|Casting|CastToBP_MainCharacter _output_get))
    (Game|SpawnActorfromClass "/Game/Collab2024/Tech/IndividualWork/JoeyLayton/Reactions/BP_PlayerReaction_DoubleJump.BP_PlayerReaction_DoubleJump_C" (Math|Conversions|ToTransform(Vector) "0, 0, 0") "Undefined" "MultiplyWithRoot" 0 _asbp_main_character 0)))

(event Custom|OnReact_FloatingPlatform
  ;[1 0.7426 0.3375] Floating Platform
  (Development|PrintString "Floating Platform")
  (Game|SpawnActorfromClass "/Game/Collab2024/Tech/IndividualWork/JoeyLayton/Archive/BP_FloatingPlatform.BP_FloatingPlatform_C" (Math|Conversions|ToTransform(Vector) (Transformation|GetActorLocation)) "Undefined" "MultiplyWithRoot" 0 0))

(event Custom|OnReact_StickySurface
  (Development|PrintString "Sticky Surface"))

(event Custom|OnReact_EarthRock
  ;[0.4757 1 0.09082] Big Rock
  (Development|PrintString "Earth Rock")
  (Game|SpawnActorfromClass "/Game/Collab2024/Tech/IndividualWork/JoeyLayton/Archive/BP_BigRock.BP_BigRock_C" (Math|Conversions|ToTransform(Vector) (Transformation|GetActorLocation)) "Undefined" "MultiplyWithRoot" 0 0))

(event Custom|OnReact_WindJump
  ;[0.7853 0.7734 0.849] Wind Jump
  (Development|PrintString "Wind Jump")
  ;;[1 1 1] Ensures jump can't be stacked
  (bind _outactors (Actor|GetAllActorsOfClass "/Game/Collab2024/Tech/IndividualWork/JoeyLayton/Reactions/BP_PlayerReaction_JumpBoost.BP_PlayerReaction_JumpBoost_C"))
  (if (Utilities|Array|IsEmpty _outactors)
    (bind _output_get (CallFunction|GetPlayerinArea))
    ;;[1 1 1] Spawns jump boost actor
    (bind _asbp_main_character (Utilities|Casting|CastToBP_MainCharacter _output_get))
    (Game|SpawnActorfromClass "/Game/Collab2024/Tech/IndividualWork/JoeyLayton/Reactions/BP_PlayerReaction_JumpBoost.BP_PlayerReaction_JumpBoost_C" (Math|Conversions|ToTransform(Vector) "0, 0, 0") "Undefined" "MultiplyWithRoot" 0 _asbp_main_character 0)))

(event Custom|OnReact_FireExplosion
  (Development|PrintString "Fire Explosion"))

(event Custom|OnReact_WaterBubble
  (Development|PrintString "Water Bubble"))

(event EventTick
  (params (DeltaSeconds :type Float%20%28single-precision%29))
  ;[0.922 1 0.4158] Debug Box
  (Rendering|Debug|DrawDebugBox (Transformation|GetActorLocation) (Math|Conversions|ToVector(Float) (Variables|Default|GetAOE_Size)) (Variables|Default|GetDebug%20Color) "0, 0, 0" 0.0 0.0))

(event Collision|EventActorBeginOverlap
  (params (OtherActor :type Actor%20Object%20Reference))
  ;[1 0.4667 0.8118] Check for reaction
  (if (not (Variables|Default|GetIs%20Reacting))
    (bind _output_get (Variables|Default|SetHit%20Actor OtherActor))
    (if (Utilities|DoesObjectImplementInterface _output_get "/Game/Collab2024/Tech/CoreItems/Interfaces/BPI_Reactive.BPI_Reactive_C")
      (if (> (Actor|GetGameTimeSinceCreation (Variables|Default|GetHit%20Actor)) (Actor|GetGameTimeSinceCreation))
        (bind _asbpi_reactive (Utilities|Casting|CastToBPI_Reactive (Variables|Default|GetHit%20Actor)))
        (Default|OnReact _asbpi_reactive self)
        (else
          (CallFunction|OnReact (Variables|Default|GetHit%20Actor))
          (Variables|Default|SetIs%20Reacting true))))))

(event EventBeginPlay
  ;[1 1 1] Setup
  (bind _returnvalue (AddComponent|AddBoxComponent false))
  (Components|Box|SetBoxExtent _returnvalue (Math|Conversions|ToVector(Float) (Variables|Default|GetAOE_Size)) true)
  (Niagara|SpawnSystemAttached (Variables|Default|GetNiagaraSplashParticles) (Variables|Default|GetDefaultSceneRoot) "None" "0, 0, 0" "0, 0, 0" "KeepRelativeOffset" false)
  (Utilities|FlowControl|Delay (Variables|Default|GetAOE_Particle_Duration))
  (Actor|DestroyActor))

(event EventOnReact
  (params (ReactiveActor :type Actor%20Object%20Reference))
  ;[0 0.1647 1] Reaction type
  (bind _output_get (Variables|Default|SetReactive%20Actor ReactiveActor))
  (bind _actorelementtype (Class|BPIReactive|GetElementType(Message) _output_get))
  (Variables|Default|SetHit%20Element _actorelementtype)
  (switch Utilities|FlowControl|Switch|SwitchonEnum_ActiveElement (Variables|Default|GetElement)
    (:Fire
      (switch Utilities|FlowControl|Switch|SwitchonEnum_ActiveElement (Variables|Default|GetHit%20Element)
        (:Fire
          (CallFunction|OnReactFireExplosion))
        (:Wind
          (CallFunction|OnReactBlast :!label _label))
        (:Water
          (CallFunction|OnReactDoubleJump :!label _label_2))
        (:Earth
          (CallFunction|OnReactObsidianorMeteorite :!label _label_3))))
    (:Wind
      (switch Utilities|FlowControl|Switch|SwitchonEnum_ActiveElement (Variables|Default|GetHit%20Element)
        (:Fire
          (goto _label))
        (:Wind
          (CallFunction|OnReactWindJump))
        (:Water
          (CallFunction|OnReactSpeedBoost :!label _label_4))
        (:Earth
          (CallFunction|OnReactFloatingPlatform :!label _label_5))))
    (:Water
      (switch Utilities|FlowControl|Switch|SwitchonEnum_ActiveElement (Variables|Default|GetHit%20Element)
        (:Fire
          (goto _label_2))
        (:Wind
          (goto _label_4))
        (:Water
          (CallFunction|OnReactWaterBubble))
        (:Earth
          (CallFunction|OnReactStickySurface :!label _label_6))))
    (:Earth
      (switch Utilities|FlowControl|Switch|SwitchonEnum_ActiveElement (Variables|Default|GetHit%20Element)
        (:Fire
          (goto _label_3))
        (:Wind
          (goto _label_5))
        (:Water
          (goto _label_6))
        (:Earth
          (CallFunction|OnReactEarthRock)))))
  (Actor|DestroyActor (Variables|Default|GetReactive%20Actor))
  (Actor|DestroyActor))

(fn ConstructionScript)

(fn GetMoveableinArea
  (bind _outactors (Collision|SphereOverlapActors (Transformation|GetActorLocation) (* (Variables|Default|GetAOE_Size) 2.0) (Utilities|Array|MakeArray "ObjectTypeQuery3" "ObjectTypeQuery1" "ObjectTypeQuery2" "ObjectTypeQuery6") 0))
  (for _array_element _outactors
    (if (Utilities|DoesObjectImplementInterface _array_element "/Game/Collab2024/Tech/CoreItems/Interfaces/BPI_Moveable.BPI_Moveable_C")
      (if (Class|GameplayStatics|ObjectIsA _array_element "/Game/Collab2024/Tech/CoreItems/BP_MainCharacter.BP_MainCharacter_C")
        (LocalVariables|SetPlayerRef _array_element)
        (else
          (Utilities|Array|Add (LocalVariables|GetOutActors) _array_element)))))
  (return (LocalVariables|GetOutActors) (LocalVariables|GetPlayerRef)))

(fn GetPlayerinArea
  (bind _outactors (Collision|SphereOverlapActors (Transformation|GetActorLocation) (* (Variables|Default|GetAOE_Size) 2.0) (Utilities|Array|MakeArray "ObjectTypeQuery3") 0))
  (for _array_element _outactors
    (if (Class|GameplayStatics|ObjectIsA _array_element "/Game/Collab2024/Tech/CoreItems/BP_MainCharacter.BP_MainCharacter_C")
      (LocalVariables|SetPlayerRef _array_element)))
  (return (LocalVariables|GetPlayerRef)))

(fn GetElementType
  (return (Variables|Default|GetElement)))