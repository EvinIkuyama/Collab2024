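; Enemy homing missile projectile that steers toward the player character and destroys itself when it hits one.
; LockOn sets the movement component's homing target via FindHomingTarget, then starts a looping half-second timer that repeats the search and sets the timer again.
; The search returns a player scene component only when the player is nearer than the stored closest distance, which it then lowers.
; Destruction clears the stored timer.
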(event Custom|LockOn
  (bind _homing_target (CallFunction|FindHomingTarget))
  (Variables|/Script/Engine.ProjectileMovementComponent|SetHomingTargetComponent (Variables|Default|GetProjectileMovement) _homing_target)
  (bind _returnvalue (Utilities|Time|SetTimerbyEvent (delegate Custom|Loop) 0.5 true))
  (Variables|Default|SetLoopTimer _returnvalue))

(event Custom|Loop
  (bind _homing_target (CallFunction|FindHomingTarget))
  (Variables|/Script/Engine.ProjectileMovementComponent|SetHomingTargetComponent (Variables|Default|GetProjectileMovement) _homing_target)
  (bind _returnvalue (Utilities|Time|SetTimerbyEvent (delegate Custom|Loop) 0.5 true))
  (Variables|Default|SetLoopTimer _returnvalue))

(event EventBeginPlay)

(event Collision|EventActorBeginOverlap
  (params (OtherActor :type Actor%20Object%20Reference)))

(event EventTick
  (params (DeltaSeconds :type Float%20%28single-precision%29)))

(event Collision|EventHit
  (params (MyComp :type Primitive%20Component%20Object%20Reference) (Other :type Actor%20Object%20Reference) (OtherComp :type Primitive%20Component%20Object%20Reference) (bSelfMoved :type Boolean) (HitLocation :type Vector :default "0, 0, 0") (HitNormal :type Vector :default "0, 0, 0") (NormalImpulse :type Vector :default "0, 0, 0") (Hit :type Hit%20Result%20Structure%20%28by%20ref%29))
  (Utilities|Casting|CastToBP_MainCharacter Other)
  (Actor|DestroyActor))

(event EventDestroyed
  (Utilities|Time|ClearandInvalidateTimerbyHandle (Variables|Default|GetLoopTimer)))

(fn ConstructionScript
  (|CallParentFunction))

(fn FindHomingTarget
  (bind _returnvalue (Game|GetPlayerCharacter 0))
  (bind _returnvalue_2 (Transformation|GetActorLocation))
  (bind _returnvalue_3 (Transformation|GetActorLocation _returnvalue))
  (bind _returnvalue_4 (- _returnvalue_3 _returnvalue_2))
  (bind _returnvalue_5 (Math|Vector|VectorLength _returnvalue_4))
  (if (< _returnvalue_5 (Variables|Default|GetClosestDistance))
    (Variables|Default|SetClosestDistance _returnvalue_5)
    (Variables|Default|SetHomingTarget (Game|GetPlayerCharacter 0))
    (return (Actor|GetComponentbyClass (Variables|Default|GetHomingTarget) "/Script/Engine.SceneComponent"))))