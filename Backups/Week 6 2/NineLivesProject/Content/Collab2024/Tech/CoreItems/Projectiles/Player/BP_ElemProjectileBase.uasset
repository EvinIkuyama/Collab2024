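; Base player projectile for elemental attacks, with exposed element, splash particle, duration and area variables for child Blueprints.
; On hit it plays a glass-smash sound, fires a surface-hit dispatcher, spawns a BP_ElementSplashAndReaction configured from those variables, then destroys itself.
; Collision overlaps send the other actor an OnInteract interface message matching the Wind, Fire or Water element, so only implementers respond.
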(event OnComponentBeginOverlap(CollisionComponent)
  (params (OverlappedComponent :type Primitive%20Component%20Object%20Reference) (OtherActor :type Actor%20Object%20Reference) (OtherComp :type Primitive%20Component%20Object%20Reference) (OtherBodyIndex :type Integer) (bFromSweep :type Boolean) (SweepResult :type Hit%20Result%20Structure%20%28by%20ref%29))
  ;[1 1 1] Calls on interact if the hit actor utilises the interface
  (switch Utilities|FlowControl|Switch|SwitchonEnum_ActiveElement (Variables|Default|GetElement)
    (:Wind
      (Class|BPIInteractable|OnInteract(Message) OtherActor "NewEnumerator0"))
    (:Fire
      (Class|BPIInteractable|OnInteract(Message) OtherActor "NewEnumerator1"))
    (:Water
      (Class|BPIInteractable|OnInteract(Message) OtherActor "NewEnumerator2"))))

(event Collision|EventHit
  (params (MyComp :type Primitive%20Component%20Object%20Reference) (Other :type Actor%20Object%20Reference) (OtherComp :type Primitive%20Component%20Object%20Reference) (bSelfMoved :type Boolean) (HitLocation :type Vector :default "0, 0, 0") (HitNormal :type Vector :default "0, 0, 0") (NormalImpulse :type Vector :default "0, 0, 0") (Hit :type Hit%20Result%20Structure%20%28by%20ref%29))
  (Audio|PlaySoundatLocation "/Game/TemplateAssets/FPWeapon/Audio/glass_bottle_smash.glass_bottle_smash" HitLocation "0, 0, 0" 1.0 1.0 0.0 0 0 0 0) ; Play smash sound
  (Default|CallOnProjectileHitSurface)
  (Game|SpawnActorfromClass "/Game/Collab2024/Tech/IndividualWork/JoeyLayton/BP_ElementSplashAndReaction.BP_ElementSplashAndReaction_C" (Transformation|GetActorTransform) "Undefined" "MultiplyWithRoot" 0 (Variables|Default|GetNiagara%20Splash%20Particles) (Variables|Default|GetAOE_Splash_Duration) (Variables|Default|GetAOE%20Size) (Variables|Default|GetElement) 0)
  (Actor|DestroyActor))

(fn ConstructionScript)