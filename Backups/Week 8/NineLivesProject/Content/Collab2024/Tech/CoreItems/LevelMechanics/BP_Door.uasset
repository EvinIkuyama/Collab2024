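; BP_Door is a level mechanic actor that slides to a target location when a connected button triggers it.
; MoveDoor runs once, guarded by a DoorOpened flag, and caches the current position as the start.
; A DoorMovement timeline then lerps the actor from that start to NewLocation without sweeping, and the door has no closing logic.
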(event Custom|MoveDoor
  ;[1 1 1] When connected button is hit, move to specified location
  (if (not (Variables|Default|GetDoorOpened))
    (Variables|Default|SetDoorOpened true)
    (Variables|Default|SetStartLocation (Transformation|GetActorLocation))
    (bind _alpha (Timeline|DoorMovement Play)
      (:Update
        (Transformation|SetActorLocation (Math|Vector|Lerp(Vector) (Variables|Default|GetStartLocation) (Variables|Default|GetNewLocation) _alpha) false false)))))

(fn ConstructionScript)