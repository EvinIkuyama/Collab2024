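; BP_IcePath is a level mechanic that overrides the player character's walk speed while it overlaps an active ice path.
; Box overlap starts a looping timer that applies the ice speed, caching the original speed once on the first tick.
; A Fire interaction deactivates the ice, despite a note saying earth.
; Leaving the box, or a tick finding the ice inactive, restores the cached speed and clears the timer.
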(event OnComponentBeginOverlap(Box)
  (params (OverlappedComponent :type Primitive%20Component%20Object%20Reference) (OtherActor :type Actor%20Object%20Reference) (OtherComp :type Primitive%20Component%20Object%20Reference) (OtherBodyIndex :type Integer) (bFromSweep :type Boolean) (SweepResult :type Hit%20Result%20Structure%20%28by%20ref%29))
  ;[1 1 1] Loops ice active check and speed changes on overlap
  (bind _asbp_main_character (Utilities|Casting|CastToBP_MainCharacter OtherActor))
  (Variables|Default|SetPlayerCharacter _asbp_main_character)
  (bind _returnvalue (Utilities|Time|SetTimerbyEvent (delegate Custom|SetPlayerSpeed) 0.1 true))
  (Variables|Default|SetTimerHandle _returnvalue))

(event OnComponentEndOverlap(Box)
  (params (OverlappedComponent :type Primitive%20Component%20Object%20Reference) (OtherActor :type Actor%20Object%20Reference) (OtherComp :type Primitive%20Component%20Object%20Reference) (OtherBodyIndex :type Integer))
  ;[1 1 1] Sets speed to normal after collision end and stops loop
  (if (== OtherActor (Variables|Default|GetPlayerCharacter))
    (Utilities|Time|ClearandInvalidateTimerbyHandle (Variables|Default|GetTimerHandle))
    (Variables|/Script/Engine.CharacterMovementComponent|SetMaxWalkSpeed (Variables|/Script/Engine.Character|GetCharacterMovement (Variables|Default|GetPlayerCharacter)) (Variables|Default|GetMaxWalkSpeedDefault))))

(event Custom|SetPlayerSpeed
  (bind _playercharacter (Variables|Default|GetPlayerCharacter))
  (bind _charactermovement (Variables|/Script/Engine.Character|GetCharacterMovement _playercharacter))
  ;[1 1 1] Checks if the path still has ice active and sets the player speed appropriately
  (Utilities|FlowControl|Sequence
    (:then_0
      (Utilities|FlowControl|DoOnce false
        (:Completed
          (Variables|Default|SetMaxWalkSpeedDefault (Variables|/Script/Engine.CharacterMovementComponent|GetMaxWalkSpeed _charactermovement)))))
    (:then_1
      (if (Variables|Default|GetIceActive)
        (Variables|/Script/Engine.CharacterMovementComponent|SetMaxWalkSpeed _charactermovement 5e+02)
        (else
          (Variables|/Script/Engine.CharacterMovementComponent|SetMaxWalkSpeed _charactermovement (Variables|Default|GetMaxWalkSpeedDefault))
          (Utilities|Time|ClearandInvalidateTimerbyHandle (Variables|Default|GetTimerHandle)))))))

(event EventOnInteract
  (params (Element :type Enum_ActiveElement%20Enum :default "Fire"))
  ;[1 1 1] Sets ice active to false when hit with the earth element
  (switch Utilities|FlowControl|Switch|SwitchonEnum_ActiveElement Element
    (:Fire
      (Variables|Default|SetIceActive false))))

(fn ConstructionScript)