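; Elemental splash area for Fire, Wind or Water that combines with another splash on overlap to create a player reaction.
; BeginPlay adds a box volume and, without a direct splash, shows Niagara particles before expiring after the AOE duration.
; The first overlap locks reacting; against an older reactive splash, the newer one destroys both and spawns an order-independent element-pair effect.
; Tick draws the area as a debug box.
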(event Custom|Destroy%20System
  (bind _particle_system (Variables|Default|GetParticle%20System))
  ;[1 1 1] Remove Particle System
  (Utilities|IsValid _particle_system
    (:Is%20Valid
      (Components|DestroyComponent _particle_system))))

(event Custom|Deactivate%20System
  (bind _particle_system (Variables|Default|GetParticle%20System))
  ;[1 1 1] Remove Particle System
  (Utilities|IsValid _particle_system
    (:Is%20Valid
      (Components|Activation|Deactivate _particle_system))))

(event Custom|SpawnSystem
  ;[1 1 1] Niagara Spawn
  (bind _returnvalue (Niagara|SpawnSystematLocation (Variables|Default|GetNiagaraSplashParticles) (Transformation|GetActorLocation)))
  (Variables|Default|SetParticle%20System _returnvalue))

(event EventTick
  (params (DeltaSeconds :type Float%20%28single-precision%29))
  (bind _aoe_size (Variables|Default|GetAOE%20Size))
  ;[1 1 1] Setup
  ;;[1 1 1] Collision Box
  ;;;[1 0.6184 0] Debug Box
  (Rendering|Debug|DrawDebugBox (Transformation|GetActorLocation) (Math|Vector|MakeVector _aoe_size _aoe_size (Variables|Default|GetAOE%20Height)) "(R=1.000000,G=1.000000,B=1.000000,A=1.000000)" "0, 0, 0" 0.0 0.0))

(event Collision|EventActorBeginOverlap
  (params (OtherActor :type Actor%20Object%20Reference))
  ;[1 0.4667 0.8118] Check for reaction
  (if (not (Variables|Default|GetIs%20Reacting?))
    (Variables|Default|SetIs%20Reacting? true)
    (bind _output_get (Variables|Default|SetHit%20Actor OtherActor))
    (if (Utilities|DoesObjectImplementInterface _output_get "/Game/Collab2024/Tech/CoreItems/Interfaces/BPI_Reactive.BPI_Reactive_C")
      (Variables|Default|SetDirect%20Splash true)
      (if (> (Actor|GetGameTimeSinceCreation (Variables|Default|GetHit%20Actor)) (Actor|GetGameTimeSinceCreation))
        (CallFunction|OnReact (Variables|Default|GetHit%20Actor))))))

(event EventBeginPlay
  (bind _aoe_size (Variables|Default|GetAOE%20Size))
  ;[1 1 1] Setup
  ;;[1 1 1] Collision Box
  (bind _returnvalue (AddComponent|AddBoxComponent false))
  (Components|Box|SetBoxExtent _returnvalue (Math|Vector|MakeVector _aoe_size _aoe_size (Variables|Default|GetAOE%20Height)) true)
  (if (not (Variables|Default|GetDirect%20Splash))
    (CallFunction|SpawnSystem)
    (Utilities|FlowControl|Delay (Variables|Default|GetAOE%20Duration))
    (CallFunction|DeactivateSystem)
    (Actor|DestroyActor)))

(event EventOnReact
  (params (ReactiveActor :type Actor%20Object%20Reference))
  ;[0 0.1647 1] Reaction
  (bind _asbp_element_splash_and_reaction (Utilities|Casting|CastToBP_ElementSplashAndReaction ReactiveActor))
  (CallFunction|DestroySystem _asbp_element_splash_and_reaction)
  (CallFunction|DestroySystem)
  (bind _actorelementtype (Class|BPIReactive|GetElementType(Message) _asbp_element_splash_and_reaction))
  (switch Utilities|FlowControl|Switch|SwitchonEnum_ActiveElement _actorelementtype
    (:Fire
      (Actor|DestroyActor _asbp_element_splash_and_reaction)
      (switch Utilities|FlowControl|Switch|SwitchonEnum_ActiveElement (Variables|Default|GetElement)
        (:Fire
          (CallFunction|SpawnEffectandSelfDestruct "/Game/Collab2024/Tech/IndividualWork/JoeyLayton/Reactions/BP_PlayerReaction_FireFire.BP_PlayerReaction_FireFire_C"))
        (:Wind
          (CallFunction|SpawnEffectandSelfDestruct "/Game/Collab2024/Tech/IndividualWork/JoeyLayton/Reactions/BP_PlayerReaction_FireWind.BP_PlayerReaction_FireWind_C" :!label _label))
        (:Water
          (CallFunction|SpawnEffectandSelfDestruct "/Game/Collab2024/Tech/IndividualWork/JoeyLayton/Reactions/BP_PlayerReaction_WaterFire.BP_PlayerReaction_WaterFire_C" :!label _label_2))))
    (:Wind
      (Actor|DestroyActor _asbp_element_splash_and_reaction)
      (switch Utilities|FlowControl|Switch|SwitchonEnum_ActiveElement (Variables|Default|GetElement)
        (:Fire
          (goto _label))
        (:Wind
          (CallFunction|SpawnEffectandSelfDestruct "/Game/Collab2024/Tech/IndividualWork/JoeyLayton/Reactions/BP_PlayerReaction_WindWind.BP_PlayerReaction_WindWind_C"))
        (:Water
          (CallFunction|SpawnEffectandSelfDestruct "/Game/Collab2024/Tech/IndividualWork/JoeyLayton/Reactions/BP_PlayerReaction_WaterWind.BP_PlayerReaction_WaterWind_C" :!label _label_3))))
    (:Water
      (Actor|DestroyActor _asbp_element_splash_and_reaction)
      (switch Utilities|FlowControl|Switch|SwitchonEnum_ActiveElement (Variables|Default|GetElement)
        (:Fire
          (goto _label_2))
        (:Wind
          (goto _label_3))
        (:Water
          (CallFunction|SpawnEffectandSelfDestruct "/Game/Collab2024/Tech/IndividualWork/JoeyLayton/Reactions/BP_PlayerReaction_WaterWater.BP_PlayerReaction_WaterWater_C"))))))

(fn ConstructionScript)

(fn SpawnEffectandSelfDestruct
  (params (Reaction%20Actor%20Reference :type Actor%20Class%20Reference))
  (Game|SpawnActorfromClass Reaction%20Actor%20Reference (Transformation|GetActorTransform) "Undefined" "MultiplyWithRoot" 0 0)
  (CallFunction|DestroySystem)
  (Actor|DestroyActor))

(fn GetElementType
  (return (Variables|Default|GetElement)))