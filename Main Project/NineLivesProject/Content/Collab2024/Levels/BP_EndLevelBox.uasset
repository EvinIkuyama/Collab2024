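; BP_EndLevelBox is a level-end trigger that finishes a speedrun when any actor begins overlapping it.
; On overlap it gets BP_GM_MainMode, stops its BP_SpeedrunTimer, and passes the truncated total time to the game mode's GradeSystem for a grade.
; It then creates WBP_EndLevelScreen, adds it to the viewport, and fills in the time and grade text.
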(event EventBeginPlay)

(event Collision|EventActorBeginOverlap
  (params (OtherActor :type Actor%20Object%20Reference))
  (bind _asbp_gm_main_mode (Utilities|Casting|CastToBP_GM_MainMode (Game|GetGameMode))
    (:then
      (Variables|Default|SetAs%20BP%20GM%20Main%20Mode _asbp_gm_main_mode)
      (Default|Stop (Actor|GetComponentbyClass _asbp_gm_main_mode "/Game/Collab2024/Tech/IndividualWork/EvinOxley/BP_SpeedrunTimer.BP_SpeedrunTimer_C"))
      (bind _returnvalue (Class|GradeSystem|PlayerGrade (Variables|/Game/Collab2024/Tech/CoreItems/BP_GM_MainMode.BP_GM_MainMode_C|GetGradeSystem (Variables|Default|GetAs%20BP%20GM%20Main%20Mode)) (Math|Float|Truncate (Variables|/Game/Collab2024/Tech/IndividualWork/EvinOxley/BP_SpeedrunTimer.BP_SpeedrunTimer_C|GettotalTime (Actor|GetComponentbyClass _asbp_gm_main_mode "/Game/Collab2024/Tech/IndividualWork/EvinOxley/BP_SpeedrunTimer.BP_SpeedrunTimer_C")))))
      (Development|PrintString _returnvalue)
      (bind _returnvalue_2 (UserInterface|CreateWidget "/Game/Collab2024/Tech/IndividualWork/TomLawrence/UI/WBP_EndLevelScreen.WBP_EndLevelScreen_C"))
      (bind _output_get (Variables|Default|SetEndLevelScreen _returnvalue_2))
      (UserInterface|Viewport|AddtoViewport _output_get 0)
      (Rendering|Components|TextRender|SetText (Variables|/Game/Collab2024/Tech/IndividualWork/TomLawrence/UI/WBP_EndLevelScreen.WBP_EndLevelScreen_C|GetText_Timer (Variables|Default|GetEndLevelScreen)) (Utilities|Text|ToText(Float) (Variables|/Game/Collab2024/Tech/IndividualWork/EvinOxley/BP_SpeedrunTimer.BP_SpeedrunTimer_C|GettotalTime (Actor|GetComponentbyClass _asbp_gm_main_mode "/Game/Collab2024/Tech/IndividualWork/EvinOxley/BP_SpeedrunTimer.BP_SpeedrunTimer_C")) "HalfToEven" false true 1 324 0 2))
      (Rendering|Components|TextRender|SetText (Variables|/Game/Collab2024/Tech/IndividualWork/TomLawrence/UI/WBP_EndLevelScreen.WBP_EndLevelScreen_C|GetText_Grade (Variables|Default|GetEndLevelScreen)) (Utilities|Text|ToText(String) _returnvalue)))
    (:CastFailed
      (Development|PrintString "Failed to stop timer"))))

(event EventTick
  (params (DeltaSeconds :type Float%20%28single-precision%29)))

(fn ConstructionScript)