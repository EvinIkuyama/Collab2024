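; Elemental splash actor that spawns a timed area of effect with Niagara particles and combines with overlapping reactive actors.
; BeginPlay adds a sphere, box or capsule collider, which Tick debug-draws.
; On overlap, only the younger actor reacts, mapping both elements (Wind, Fire, Water, Earth) to an order-independent reaction, then destroying both.
; Only Blast is implemented, launching nearby moveable pawns with separate player and enemy impulses; other reactions are print-string stubs.
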(event Custom|OnReact_Blast
  ;[1 0.3534 0.3833] Explosion
  (Development|PrintString "Blast")
  (Niagara|SpawnSystematLocation "/Game/Collab2024/Tech/NiagaraEffects/PS_Elem_Explosion.PS_Elem_Explosion" (Transformation|GetActorLocation))
  (bind _outactors (Collision|SphereOverlapActors (Transformation|GetActorLocation) (* (Variables|Default|GetAOE_Size) 2.0) (Utilities|Array|MakeArray "ObjectTypeQuery3") 0))
  (for _array_element _outactors
    (if (Utilities|DoesObjectImplementInterface _array_element "/Game/Collab2024/Tech/CoreItems/Interfaces/BPI_Moveable.BPI_Moveable_C")
      (Utilities|Array|Add (Variables|Default|GetMoveableActors) _array_element)))
  (for _array_element_2 (Variables|Default|GetMoveableActors)
    (bind _asbp_main_character (Utilities|Casting|CastToBP_MainCharacter _array_element_2)
      (:then
        ;;[1 1 1] Player Impulse
        (Physics|AddImpulse (Variables|/Script/Engine.Character|GetCharacterMovement _asbp_main_character) (+ (* (Math|Vector|Normalize (Transformation|GetVelocity)) (Math|Conversions|ToVector(Float) 1e+02)) (* (Math|Vector|MakeVector 0.0 0.0 1e+02) (Math|Conversions|ToVector(Float) 1e+03))) false))
      (:CastFailed
        ;;[1 1 1] Enemy Impulse
        (Physics|AddImpulse (Actor|GetComponentbyClass _array_element_2 "/Script/Engine.PrimitiveComponent") (+ (* (Math|Vector|Normalize (- (Transformation|GetActorLocation _array_element_2) (Transformation|GetActorLocation))) (Math|Conversions|ToVector(Float) 1e+03)) "0.000000,0.000000,200.000000") "None" true)))))

(event Custom|OnReact_SpeedBoost
  (Development|PrintString "Speed Boost"))

(event Custom|OnReact_ObsidianOrMeteorite
  (Development|PrintString "Obsidian or Meteorite"))

(event Custom|OnReact_DoubleJump
  (Development|PrintString "Double Jump"))

(event Custom|OnReact_FloatingPlatform
  (Development|PrintString "Floating Platform"))

(event Custom|OnReact_StickySurface
  (Development|PrintString "Sticky Surface"))

(event Custom|OnReact_EarthRock
  (Development|PrintString "Earth Rock"))

(event Custom|OnReact_WindJump
  (Development|PrintString "Wind Jump"))

(event Custom|OnReact_FireExplosion
  (Development|PrintString "Fire Explosion"))

(event Custom|OnReact_WaterBubble
  (Development|PrintString "Water Bubble"))

(event EventTick
  (params (DeltaSeconds :type Float%20%28single-precision%29))
  ;[0.922 1 0.4158] Debugging
  (switch Utilities|FlowControl|Switch|SwitchonEnum_AOEType (Variables|Default|GetAOE_Type)
    (:NewEnumerator0
      (Rendering|Debug|DrawDebugSphere (Transformation|GetActorLocation) (Variables|Default|GetAOE_Size) 12 (Variables|Default|GetDebug%20Color) 0.0))
    (:NewEnumerator1
      (Rendering|Debug|DrawDebugBox (Transformation|GetActorLocation) (Math|Conversions|ToVector(Float) (Variables|Default|GetAOE_Size)) (Variables|Default|GetDebug%20Color) "0, 0, 0" 0.0 0.0))
    (:NewEnumerator2
      (Rendering|Debug|DrawDebugCapsule (Transformation|GetActorLocation) 0.0 (Variables|Default|GetAOE_Size) "0, 0, 0" (Variables|Default|GetDebug%20Color) 0.0 0.0))))

(event Collision|EventActorBeginOverlap
  (params (OtherActor :type Actor%20Object%20Reference))
  ;[1 0.4667 0.8118] Check for reaction
  (if (not (Variables|Default|GetIs%20Reacting))
    (bind _output_get (Variables|Default|SetHit%20Actor OtherActor))
    (if (Utilities|DoesObjectImplementInterface _output_get "/Game/Collab2024/Tech/CoreItems/Interfaces/BPI_Reactive.BPI_Reactive_C")
      (if (> (Actor|GetGameTimeSinceCreation (Variables|Default|GetHit%20Actor)) (Actor|GetGameTimeSinceCreation))
        (CallFunction|OnReact (Variables|Default|GetHit%20Actor))
        (Variables|Default|SetIs%20Reacting true)))))

(event EventBeginPlay
  ;[1 1 1] Setup
  (switch Utilities|FlowControl|Switch|SwitchonEnum_AOEType (Variables|Default|GetAOE_Type)
    (:NewEnumerator0
      (bind _returnvalue (AddComponent|AddSphereComponent false))
      (Components|Sphere|SetSphereRadius _returnvalue (Variables|Default|GetAOE_Size) true))
    (:NewEnumerator1
      (bind _returnvalue_2 (AddComponent|AddBoxComponent false))
      (Components|Box|SetBoxExtent _returnvalue_2 (Math|Conversions|ToVector(Float) (Variables|Default|GetAOE_Size)) true))
    (:NewEnumerator2
      (bind _returnvalue_3 (AddComponent|AddCapsuleComponent false))
      (Components|Capsule|SetCapsuleRadius _returnvalue_3 (Variables|Default|GetAOE_Size) true)))
  (Niagara|SpawnSystemAttached (Variables|Default|GetNiagaraSplashParticles) (Variables|Default|GetDefaultSceneRoot) "None" "0, 0, 0" "0, 0, 0" "KeepRelativeOffset" false)
  (Utilities|FlowControl|Delay (Variables|Default|GetAOE_Particle_Duration))
  (Actor|DestroyActor))

(event EventOnReact
  (params (ReactiveActor :type Actor%20Object%20Reference))
  ;[0 0.1647 1] Reaction type
  (bind _output_get (Variables|Default|SetReactive%20Actor ReactiveActor))
  (bind _actorelementtype (Class|BPIReactive|GetElementType(Message) _output_get))
  (Variables|Default|SetHit%20Element _actorelementtype)
  (switch Utilities|FlowControl|Switch|SwitchonEnum_ActiveElement (Variables|Default|GetElement)
    (:Wind
      (switch Utilities|FlowControl|Switch|SwitchonEnum_ActiveElement (Variables|Default|GetHit%20Element)
        (:Wind
          (CallFunction|OnReactWindJump))
        (:Fire
          (CallFunction|OnReactBlast :!label _label))
        (:Water
          (CallFunction|OnReactSpeedBoost :!label _label_2))
        (:Earth
          (CallFunction|OnReactFloatingPlatform :!label _label_3))))
    (:Fire
      (switch Utilities|FlowControl|Switch|SwitchonEnum_ActiveElement (Variables|Default|GetHit%20Element)
        (:Wind
          (goto _label))
        (:Fire
          (CallFunction|OnReactFireExplosion))
        (:Water
          (CallFunction|OnReactDoubleJump :!label _label_4))
        (:Earth
          (CallFunction|OnReactObsidianorMeteorite :!label _label_5))))
    (:Water
      (switch Utilities|FlowControl|Switch|SwitchonEnum_ActiveElement (Variables|Default|GetHit%20Element)
        (:Wind
          (goto _label_2))
        (:Fire
          (goto _label_4))
        (:Water
          (CallFunction|OnReactWaterBubble))
        (:Earth
          (CallFunction|OnReactStickySurface :!label _label_6))))
    (:Earth
      (switch Utilities|FlowControl|Switch|SwitchonEnum_ActiveElement (Variables|Default|GetHit%20Element)
        (:Wind
          (goto _label_3))
        (:Fire
          (goto _label_5))
        (:Water
          (goto _label_6))
        (:Earth
          (CallFunction|OnReactEarthRock)))))
  (Actor|DestroyActor (Variables|Default|GetReactive%20Actor))
  (Actor|DestroyActor))

(fn ConstructionScript)

(fn GetElementType
  (return (Variables|Default|GetElement)))