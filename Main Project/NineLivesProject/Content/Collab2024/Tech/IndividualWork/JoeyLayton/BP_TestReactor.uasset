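; BP_TestReactor is a test actor for elemental reactions, with a cube meant to resize in response to reactive actors.
; OnReact prints a debug message, queries the incoming actor's element, runs an element switch, then destroys that actor.
; The switch's Fire branch halves the cube's scale and Water doubles it, bounded by a min/max step counter; Wind and Earth do nothing.
; The reactor reports its own element as Wind.
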(event Custom|OnShrink
  (bind _cube (Variables|Default|GetCube))
  (bind _returnvalue (Transformation|GetWorldTransform _cube))
  (bind (_location _rotation _scale) (Math|Transform|BreakTransform _returnvalue))
  ;[1 1 1] Shrink
  (if (> (Variables|Default|GetCube%20Size) (Variables|Default|GetMin%20Cube%20Size))
    (Transformation|SetWorldTransform (Variables|Default|GetCube) (Math|Transform|MakeTransform _location _rotation (/ _scale "2.000000,2.000000,2.000000")) false false)
    (Math|Integer|DecrementInt (Variables|Default|GetCube%20Size))))

(event Custom|OnGrow
  (bind _cube (Variables|Default|GetCube))
  (bind _returnvalue (Transformation|GetWorldTransform _cube))
  (bind (_location _rotation _scale) (Math|Transform|BreakTransform _returnvalue))
  ;[1 1 1] Shrink
  (if (< (Variables|Default|GetCube%20Size) (Variables|Default|GetMax%20Cube%20Size))
    (Transformation|SetWorldTransform (Variables|Default|GetCube) (Math|Transform|MakeTransform _location _rotation (* _scale "2.000000,2.000000,2.000000")) false false)
    (Math|Integer|IncrementInt (Variables|Default|GetCube%20Size))))

(event EventOnReact
  (params (ReactiveActor :type Actor%20Object%20Reference))
  (Variables|Default|SetReactive%20Actor ReactiveActor)
  (Development|PrintString "Test Reaction")
  (Class|BPIReactive|GetElementType(Message) (Variables|Default|GetReactive%20Actor))
  (switch Utilities|FlowControl|Switch|SwitchonEnum_ActiveElement "Wind"
    (:Fire
      (CallFunction|OnShrink))
    (:Wind
      _)
    (:Water
      (CallFunction|OnGrow))
    (:Earth
      _))
  (Actor|DestroyActor (Variables|Default|GetReactive%20Actor)))

(event EventBeginPlay
  (Variables|Default|SetCube%20Size 0))

(fn ConstructionScript)

(fn GetElementType
  (return 0 "Wind"))