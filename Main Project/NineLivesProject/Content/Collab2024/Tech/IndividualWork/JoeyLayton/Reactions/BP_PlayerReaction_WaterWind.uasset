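; BP_PlayerReaction_WaterWind is the player reaction for Water and Wind, a buff that temporarily raises movement speed.
; On buff start it caches the character movement's current max speed as DefaultSpeed and sets MaxWalkSpeed to that plus SpeedIncrease.
; On buff end it restores MaxWalkSpeed to the cached value.
; Timeline-driven camera FOV widening and narrowing logic is present but disconnected, so it never runs.
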(event EventBuffEvent
  (bind _player_editable (Variables|Default|GetPlayer%20Editable))
  (bind _charactermovement (Variables|/Script/Engine.Character|GetCharacterMovement _player_editable))
  ;[0.394 1 0.343] Buff Event
  ;;[1 1 1] Update speed
  (bind _output_get (Variables|Default|SetDefault%20Speed (Class|MovementComponent|GetMaxSpeed _charactermovement)))
  (Variables|/Script/Engine.CharacterMovementComponent|SetMaxWalkSpeed _charactermovement (+ _output_get (Variables|Default|GetSpeed%20Increase))))

(event EventBuffEndEvent
  ;[1 0.4374 0.4474] End Buff
  ;;[1 1 1] Update Speed
  (Variables|/Script/Engine.CharacterMovementComponent|SetMaxWalkSpeed (Variables|/Script/Engine.Character|GetCharacterMovement (Variables|Default|GetPlayer%20Editable)) (Variables|Default|GetDefault%20Speed)))

(fn ConstructionScript)