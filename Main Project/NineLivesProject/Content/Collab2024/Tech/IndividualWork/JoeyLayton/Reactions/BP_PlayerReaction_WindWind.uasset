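; BP_PlayerReaction_WindWind is a player reaction actor for a Wind-Wind reaction, meant to grant a temporary jump boost.
; Its graph caches the player's CharacterMovement JumpZVelocity, multiplies it, restores it after a delay, then destroys the actor.
; That chain has no event driving it, so it never runs as written.
; The construction script only calls the parent.
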(fn ConstructionScript
  (|CallParentFunction))