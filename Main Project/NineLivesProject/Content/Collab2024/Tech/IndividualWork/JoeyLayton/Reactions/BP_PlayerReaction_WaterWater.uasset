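; Player reaction actor for a water-plus-water combination, which sends a wave travelling forward along the camera's horizontal facing.
; On react, it turns its Box perpendicular to the camera yaw and attaches the wave particle system to it.
; A timeline moves the actor each update by an alpha-scaled step without sweeping, so speed depends on frame rate, then destroys it when finished.
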(event EventOnReact
  (Transformation|SetWorldLocationAndRotation (Variables|Default|GetBox) (Transformation|GetActorLocation) (Math|Rotator|MakeRotator 0.0 0.0 (+ (.yaw (Camera|GetCameraRotation (Game|GetPlayerCameraManager 0))) 9e+01)) false false)
  (Niagara|SpawnSystemAttached "/Game/Collab2024/Tech/IndividualWork/JoeyLayton/NiagaraEffects/PS_Wave.PS_Wave" (Variables|Default|GetBox) "None" "-30.000000,0.000000,-80.000000" "0, 0, 0" "KeepRelativeOffset" false)
  (bind _alpha (Timeline|Timeline PlayFromStart)
    (:Update
      (Transformation|SetActorRelativeLocation (+ (Transformation|GetActorLocation) (* (* _alpha 2e+01) (* (Math|Vector|GetRightVector (Variables|Default|GetBox)) (Math|Conversions|ToVector(Float) -1.0))))))
    (:Finished
      (Actor|DestroyActor))))

(fn ConstructionScript
  (|CallParentFunction))