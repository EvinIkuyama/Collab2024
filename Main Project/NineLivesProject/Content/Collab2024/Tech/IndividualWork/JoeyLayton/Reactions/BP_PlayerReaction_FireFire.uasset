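; Fire-Fire player reaction that spawns a camera-aligned flame wall, which gives a flight boost when the main character enters it.
; OnReact places the Niagara wall and orients its trigger box; it deactivates on overlap or after a set duration.
; Flight chains an FOV zoom, upward impulse and horizontal camera-forward boost without gravity, with Destructive enabled.
; When the second FOV timeline finishes, Land restores gravity and clears Destructive.
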(event Custom|Deactivate%20Wall
  (bind _flame_wall_niagara (Variables|Default|GetFlame%20Wall%20Niagara))
  (bind _box (Variables|Default|GetBox))
  ;[1 0.4509 0.3811] Deactivate Wall
  (Utilities|IsValid _flame_wall_niagara
    (:Is%20Valid
      (Components|Activation|Deactivate _flame_wall_niagara)
      (Utilities|IsValid _box
        (:Is%20Valid
          (Components|DestroyComponent _box)
          (Variables|Default|SetIs%20Disabled true))))))

(event Custom|Fly
  (bind _boost_factor (Variables|Default|GetBoost%20Factor))
  ;[1 1 1] Fly
  (bind (__player_movement __player_camera _asbp_main_character) (CallFunction|PlayerReferences))
  (bind _default_fov (CallFunction|GetFOV))
  (bind _track (Timeline|Zoom PlayFromStart)
    (:Update
      (Camera|SetFieldOfView __player_camera (- _default_fov (* (Variables|Default|GetFOV%20Change) _track))))
    (:Finished
      (Variables|/Game/Collab2024/Tech/CoreItems/BP_MainCharacter.BP_MainCharacter_C|SetbDestructive _asbp_main_character true)
      (Physics|AddImpulse __player_movement "0.000000,0.000000,500.000000" true)
      (Utilities|FlowControl|Delay 0.5)
      (Physics|AddImpulse __player_movement (* (Math|Vector|GetForwardVector __player_camera) (Math|Vector|MakeVector _boost_factor _boost_factor 0.0)) true)
      (Variables|/Script/Engine.CharacterMovementComponent|SetGravityScale __player_movement 0.0)
      (bind _default_fov_2 (CallFunction|GetFOV))
      (bind _track_2 (Timeline|Timeline PlayFromStart)
        (:Update
          (Camera|SetFieldOfView __player_camera (+ _default_fov_2 (* (Variables|Default|GetFOV%20Change) _track_2))))
        (:Finished
          (CallFunction|Land))))))

(event Custom|Land
  ;[1 1 1] Land
  (bind (__player_movement __player_camera _asbp_main_character) (CallFunction|PlayerReferences))
  (Variables|/Game/Collab2024/Tech/CoreItems/BP_MainCharacter.BP_MainCharacter_C|SetbDestructive _asbp_main_character false)
  (Variables|/Script/Engine.CharacterMovementComponent|SetGravityScale __player_movement 1.0))

(event Collision|EventActorBeginOverlap
  (params (OtherActor :type Actor%20Object%20Reference))
  ;[1 1 1] Activate Flight Buff
  (if (Class|GameplayStatics|ObjectIsA OtherActor "/Game/Collab2024/Tech/CoreItems/BP_MainCharacter.BP_MainCharacter_C")
    (CallFunction|DeactivateWall)
    (CallFunction|Fly)))

(event EventOnReact
  (bind _returnvalue (Game|GetPlayerCameraManager 0))
  (bind _returnvalue_2 (Camera|GetCameraRotation _returnvalue))
  ;[1 1 1] Setup Flame Wall
  (bind _returnvalue_3 (Niagara|SpawnSystematLocation "/Game/Collab2024/Tech/IndividualWork/JoeyLayton/NiagaraEffects/PS_Elemental_Fire_Wall.PS_Elemental_Fire_Wall" (Transformation|GetActorLocation) (Math|Rotator|MakeRotator 0.0 0.0 (+ (.yaw _returnvalue_2) 9e+01))))
  (Variables|Default|SetFlame%20Wall%20Niagara _returnvalue_3)
  (Transformation|SetWorldRotation (Variables|Default|GetBox) (Math|Rotator|MakeRotator 0.0 0.0 (.yaw _returnvalue_2)) false false)
  (Utilities|FlowControl|Delay (Variables|Default|GetWall%20Duration))
  (CallFunction|DeactivateWall)
  (if (not (Variables|Default|GetIs%20Disabled))
    (Actor|DestroyActor)))

(fn ConstructionScript
  (|CallParentFunction))

(fn PlayerReferences
  (bind _asbp_main_character (Utilities|Casting|CastToBP_MainCharacter (Game|GetPlayerCharacter 0)))
  (return (Variables|/Script/NineLivesProject.MainCharacter|Get_PlayerMovement _asbp_main_character) (Variables|/Script/NineLivesProject.MainCharacter|Get_PlayerCamera _asbp_main_character) _asbp_main_character))

(fn GetFOV
  (bind _asbp_game_instance (Utilities|Casting|CastToBP_GameInstance (Game|GetGameInstance)))
  (return (Variables|/Game/Collab2024/Tech/IndividualWork/EvinOxley/BP_GameInstance.BP_GameInstance_C|GetInsFOV _asbp_game_instance)))