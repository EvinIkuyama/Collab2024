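; Player reaction for the fire-wind combination, an explosive burst that launches the player and nearby movable actors.
; On react it spawns a burst effect, then queries the area for the player and other movable actors.
; The player gets a strong upward impulse plus current horizontal velocity, while other actors are pushed up and outward, scaled by their offset from the blast.
; Completion fires inside the per-actor loop, so only when actors are found.
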(event EventOnReact
  ;[1 0.3534 0.3833] Explosion
  (Development|PrintString "Blast")
  (Niagara|SpawnSystematLocation "/Game/Collab2024/Tech/IndividualWork/JoeyLayton/NiagaraEffects/PS_Reaction_Burst.PS_Reaction_Burst" (Transformation|GetActorLocation))
  (bind (_out_actors _player_ref) (CallFunction|GetMoveableinArea))
  ;;[1 1 1] Player Impulse
  (bind _asbp_main_character (Utilities|Casting|CastToBP_MainCharacter _player_ref)
    (:then
      (Physics|AddImpulse (Variables|/Script/Engine.Character|GetCharacterMovement _asbp_main_character) (Math|Vector|MakeVector (.X (Math|Vector|BreakVector (Transformation|GetVelocity _player_ref))) (.Y (Math|Vector|BreakVector (Transformation|GetVelocity _player_ref))) 1e+05) false))
    (:CastFailed
      _))
  ;;[1 1 1] Enemy Impulse
  (for _array_element _out_actors
    (Physics|AddImpulse (Actor|GetComponentbyClass _array_element "/Script/Engine.PrimitiveComponent") (Math|Vector|MakeVector (* 1e+03 (.X (Math|Vector|BreakVector (- (Transformation|GetActorLocation _array_element) (Transformation|GetActorLocation))))) (* (.Y (Math|Vector|BreakVector (- (Transformation|GetActorLocation _array_element) (Transformation|GetActorLocation)))) 1e+03) 5e+04) "None" false)
    (CallFunction|OnReactComplete)))

(fn ConstructionScript
  (|CallParentFunction))