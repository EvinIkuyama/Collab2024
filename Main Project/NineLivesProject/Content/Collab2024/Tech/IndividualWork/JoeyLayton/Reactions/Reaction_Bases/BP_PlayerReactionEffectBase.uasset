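; Base Blueprint for player reaction effects that provides a query for moveable actors within the effect's area.
; GetMoveableInArea runs a sphere overlap at the actor's location with a radius of twice AreaOfEffectSize, covering pawn, world and destructible object types.
; It keeps only actors implementing BPI_Moveable, returning the main character as a separate player reference and the rest as an array.
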(fn ConstructionScript
  (|CallParentFunction))

(fn GetMoveableinArea
  (bind _outactors (Collision|SphereOverlapActors (Transformation|GetActorLocation) (* (Variables|Default|GetArea%20of%20Effect%20Size) 2.0) (Utilities|Array|MakeArray "ObjectTypeQuery3" "ObjectTypeQuery1" "ObjectTypeQuery2" "ObjectTypeQuery6") 0))
  (for _array_element _outactors
    (if (Utilities|DoesObjectImplementInterface _array_element "/Game/Collab2024/Tech/CoreItems/Interfaces/BPI_Moveable.BPI_Moveable_C")
      (if (Class|GameplayStatics|ObjectIsA _array_element "/Game/Collab2024/Tech/CoreItems/BP_MainCharacter.BP_MainCharacter_C")
        (LocalVariables|SetPlayerRef _array_element)
        (else
          (Utilities|Array|Add (LocalVariables|GetOutActors) _array_element)))))
  (return (LocalVariables|GetOutActors) (LocalVariables|GetPlayerRef)))