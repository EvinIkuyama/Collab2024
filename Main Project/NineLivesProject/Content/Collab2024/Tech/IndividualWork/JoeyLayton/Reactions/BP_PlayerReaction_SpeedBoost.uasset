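; Player reaction actor that grants a temporary speed boost with a matching camera FOV widening as soon as it spawns.
; It caches the player's current max speed, raises MaxWalkSpeed by a set increase, then restores it after the boost duration.
; In parallel, timelines ease the first-person camera FOV up, hold for the same duration, then ease it back down.
; The actor destroys itself when the FOV return finishes.
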(event Custom|UpdateFOV
  ;[1 1 1] Update FOV
  (bind _output_get (Variables|Default|SetFirst%20Person%20Camera (Variables|/Game/Collab2024/Tech/CoreItems/BP_MainCharacter.BP_MainCharacter_C|GetFirstPersonCamera (Variables|Default|GetPlayer%20Reference))))
  (Variables|Default|SetDefault%20FOV (Variables|/Script/Engine.CameraComponent|GetFieldOfView _output_get))
  (bind _alpha (Timeline|TL_FOVChangeUp PlayFromStart)
    (:Update
      (Camera|SetFieldOfView (Variables|Default|GetFirst%20Person%20Camera) (+ (Variables|Default|GetDefault%20FOV) (* _alpha (Variables|Default|GetFOV%20Increase)))))
    (:Finished
      (Utilities|FlowControl|Delay (Variables|Default|GetBoost%20Duration))
      (bind _alpha_2 (Timeline|TL_FOVChangeDown PlayFromStart)
        (:Update
          (Camera|SetFieldOfView (Variables|Default|GetFirst%20Person%20Camera) (- (+ (Variables|Default|GetDefault%20FOV) (Variables|Default|GetFOV%20Increase)) (* _alpha_2 (Variables|Default|GetFOV%20Increase)))))
        (:Finished
          (Actor|DestroyActor))))))

(event Custom|Update%20Speed
  (bind _player_reference (Variables|Default|GetPlayer%20Reference))
  (bind _charactermovement (Variables|/Script/Engine.Character|GetCharacterMovement _player_reference))
  ;[1 1 1] Update speed
  (bind _output_get (Variables|Default|SetDefault%20Speed (Class|MovementComponent|GetMaxSpeed _charactermovement)))
  (Variables|/Script/Engine.CharacterMovementComponent|SetMaxWalkSpeed _charactermovement (+ _output_get (Variables|Default|GetSpeed%20Increase)))
  (Utilities|FlowControl|Delay (Variables|Default|GetBoost%20Duration))
  (Variables|/Script/Engine.CharacterMovementComponent|SetMaxWalkSpeed _charactermovement (Variables|Default|GetDefault%20Speed)))

(event EventBeginPlay
  ;[1 1 1] On spawn
  (CallFunction|UpdateFOV)
  (CallFunction|UpdateSpeed))

(fn ConstructionScript)