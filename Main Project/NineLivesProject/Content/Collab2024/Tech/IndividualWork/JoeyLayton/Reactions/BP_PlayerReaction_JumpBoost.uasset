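; BP_PlayerReaction_JumpBoost is a player reaction actor that temporarily raises the player's jump height.
; On BeginPlay it stores the referenced player's current JumpZVelocity, then sets it to that value times a multiplier.
; After the boost duration elapses, it restores the stored velocity and destroys itself, so the actor's lifetime matches the boost.
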(event EventBeginPlay
  (bind _player_reference (Variables|Default|GetPlayer%20Reference))
  (bind _charactermovement (Variables|/Script/Engine.Character|GetCharacterMovement _player_reference))
  (bind _output_get (Variables|Default|SetDefault%20Jump%20Height (Variables|/Script/Engine.CharacterMovementComponent|GetJumpZVelocity _charactermovement)))
  (Variables|/Script/Engine.CharacterMovementComponent|SetJumpZVelocity _charactermovement (* _output_get (Variables|Default|GetJump%20Increase%20Multi)))
  (Utilities|FlowControl|Delay (Variables|Default|GetBoost%20Duration))
  (Variables|/Script/Engine.CharacterMovementComponent|SetJumpZVelocity _charactermovement (Variables|Default|GetDefault%20Jump%20Height))
  (Actor|DestroyActor))

(fn ConstructionScript
  (|CallParentFunction))