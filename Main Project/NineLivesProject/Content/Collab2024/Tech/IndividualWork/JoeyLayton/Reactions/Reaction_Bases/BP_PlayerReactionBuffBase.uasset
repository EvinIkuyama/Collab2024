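; Base reaction Blueprint for player buff pickups, spawning a pickup particle system at its location when it reacts.
; Overlap by BP_MainCharacter removes the particle and checks the player's BuffsAndDebuffs array for a matching class.
; A match calls OnBuffDurationExtend, while a new buff adds its class and calls OnBuffActivate.
; Both events here go straight to OnBuffEnd, which destroys the actor, leaving no buff effect in the base.
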(event Custom|OnBuffActivate
  (CallFunction|OnBuffEnd))

(event Custom|OnBuffDurationExtend
  (CallFunction|OnBuffEnd))

(event Custom|OnBuffEnd
  (Actor|DestroyActor))

(event Collision|EventActorBeginOverlap
  (params (OtherActor :type Actor%20Object%20Reference))
  (if (Class|GameplayStatics|ObjectIsA OtherActor "/Game/Collab2024/Tech/CoreItems/BP_MainCharacter.BP_MainCharacter_C")
    (Components|DestroyComponent (Variables|Default|GetParticle%20Reference))
    (bind _buffs_reference (CallFunction|SetPlayer&PlayerBuffsRef OtherActor))
    (bind _array_element (Utilities|Array|ForEachLoopwithBreak _buffs_reference :!label _label)
      (:LoopBody
        (if (Class|GameplayStatics|ObjectIsA self _array_element)
          (Variables|Default|SetReacting true)
          (goto _label Break)))
      (:Completed
        (if (Variables|Default|GetReacting)
          (CallFunction|OnBuffDurationExtend)
          (else
            ;[1 1 1] Add Buff to Player
            (Utilities|Array|Add (Variables|Default|GetBuffs%20And%20Debuffs) (Utilities|GetClass self))
            (CallFunction|OnBuffActivate)))))))

(event EventOnReact
  (bind _returnvalue (Niagara|SpawnSystematLocation "/Game/Collab2024/Tech/IndividualWork/JoeyLayton/NiagaraEffects/PS_Buff_Pickup.PS_Buff_Pickup" (Transformation|GetActorLocation)))
  (Variables|Default|SetParticle%20Reference _returnvalue))

(fn ConstructionScript)

(fn SetPlayer&PlayerBuffsRef
  (params (Actor :type Actor%20Object%20Reference))
  (bind _asbp_main_character (Utilities|Casting|CastToBP_MainCharacter Actor))
  (bind _output_get (Variables|Default|SetPlayer%20Editable _asbp_main_character))
  (bind _output_get_2 (Variables|Default|SetBuffs%20And%20Debuffs (Variables|/Game/Collab2024/Tech/CoreItems/BP_MainCharacter.BP_MainCharacter_C|GetBuffs%20and%20Debuffs _output_get)))
  (return _output_get_2))