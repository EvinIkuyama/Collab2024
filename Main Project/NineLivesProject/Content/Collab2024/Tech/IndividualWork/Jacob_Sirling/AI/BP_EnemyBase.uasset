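; BP_EnemyBase is an enemy character base that reacts to elemental projectile hits.
; OnInteract, called from the projectile Blueprint, switches on the Fire, Wind or Water element and destroys the enemy if the matching Weaknesses value equals one.
; A separate PushBack event launches the character along a fixed world-space vector with upward lift, adding to its current velocity.
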(event EventPushBack
  (Character|LaunchCharacter "500.000000,0.000000,200.000000" false false))

(event EventOnInteract
  (params (Element :type Enum_ActiveElement%20Enum :default "Fire"))
  ;[1 1 1] Called from projectile blueprint
  (switch Utilities|FlowControl|Switch|SwitchonEnum_ActiveElement Element
    (:Fire
      ;;[1 1 1] Checks if the enemy is weak to the interacted element
      (if (== (Utilities|Struct|BreakS_EnemyWeaknesses (Variables|Default|GetWeaknesses)) 1.0)
        ;;[1 1 1] If the enemy is weak, destroys the enemy
        (Actor|DestroyActor)))
    (:Wind
      (if (== (Utilities|Struct|BreakS_EnemyWeaknesses (Variables|Default|GetWeaknesses)) 1.0)
        (Actor|DestroyActor)))
    (:Water
      (if (== (Utilities|Struct|BreakS_EnemyWeaknesses (Variables|Default|GetWeaknesses)) 1.0)
        (Actor|DestroyActor)))))

(fn ConstructionScript)