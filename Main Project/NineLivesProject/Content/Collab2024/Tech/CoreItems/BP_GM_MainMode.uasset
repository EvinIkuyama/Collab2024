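; Main game mode that boots the player and HUD and runs the speedrun timer.
; On BeginPlay it initializes the main player controller and character, creates the HUD widget, then starts the speedrun timer.
; Each Tick writes the timer's total time to the HUD's timer text.
; Custom events switch full-severity, uncorrected color vision deficiency simulation between deuteranope, protanope, tritanope and normal vision.
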(event Custom|NormalVision
  ;[1 1 1] Colourblind Events
  (Class|WidgetBlueprintLibrary|SetColorVisionDeficiencyType "NormalVision" 1.0 false))

(event Custom|DeuteranopeVision
  ;[1 1 1] Colourblind Events
  (Class|WidgetBlueprintLibrary|SetColorVisionDeficiencyType "Deuteranope" 1.0 false))

(event Custom|ProtanopeVision
  ;[1 1 1] Colourblind Events
  (Class|WidgetBlueprintLibrary|SetColorVisionDeficiencyType "Protanope" 1.0 false))

(event Custom|TritanopeVision
  ;[1 1 1] Colourblind Events
  (Class|WidgetBlueprintLibrary|SetColorVisionDeficiencyType "Tritanope" 1.0 false))

(event EventBeginPlay
  (bind _returnvalue (Game|GetPlayerController 0))
  ;[1 1 1] Event that fires at the start of the game
  (bind _asbp_pc_main_character (Utilities|Casting|CastToBP_PC_MainCharacter _returnvalue))
  (Default|Init _asbp_pc_main_character)
  (bind _asbp_main_character (Utilities|Casting|CastToBP_MainCharacter (Game|GetPlayerCharacter 0)))
  (Default|Init _asbp_main_character)
  (bind _returnvalue_2 (UserInterface|CreateWidget "/Game/Collab2024/Tech/CoreItems/UI/WBP_HUD.WBP_HUD_C" _returnvalue))
  (bind _output_get (Variables|Default|SetWBP_HUD _returnvalue_2))
  (UserInterface|Viewport|AddtoViewport _output_get 0)
  (Default|Start (Variables|Default|GetBP_SpeedrunTimer)))

(event EventTick
  (params (DeltaSeconds :type Float%20%28single-precision%29))
  ;[1 1 1] Setting the speedrun timer
  (Rendering|Components|TextRender|SetText (Variables|/Game/Collab2024/Tech/IndividualWork/TomLawrence/UI/Widgets/WBP_Timer.WBP_Timer_C|GetText_Timer (Variables|/Game/Collab2024/Tech/CoreItems/UI/WBP_HUD.WBP_HUD_C|GetWBP_Timer (Variables|Default|GetWBP_HUD))) (Utilities|Text|ToText(Float) (Variables|/Game/Collab2024/Tech/IndividualWork/EvinOxley/BP_SpeedrunTimer.BP_SpeedrunTimer_C|GettotalTime (Variables|Default|GetBP_SpeedrunTimer)) "HalfToEven" false true 1 324 0 2)))

(fn ConstructionScript)