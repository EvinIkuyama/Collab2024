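; BP_EndLevelBox is a level-exit trigger that completes the level when overlapped, provided remaining enemies are at or below RequiredNumberLeft.
; Tick counts BP_EnemyBase actors every frame to update the HUD and feed that check.
; On completion it stops the game mode's speedrun timer, grades the time, and saves results through BP_GameInstance, resetting retries.
; It then shows WBP_EndLevelScreen with the time and star grade.
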(event EventBeginPlay
  (bind _asbp_gm_main_mode (Utilities|Casting|CastToBP_GM_MainMode (Game|GetGameMode)))
  (Variables|Default|SetAs%20BP%20GM%20Main%20Mode _asbp_gm_main_mode))

(event Collision|EventActorBeginOverlap
  (params (OtherActor :type Actor%20Object%20Reference))
  (bind _as_bp_gm_main_mode (Variables|Default|GetAs%20BP%20GM%20Main%20Mode))
  (bind _returnvalue (Actor|GetComponentbyClass _as_bp_gm_main_mode "/Game/Collab2024/Tech/IndividualWork/EvinOxley/BP_SpeedrunTimer.BP_SpeedrunTimer_C"))
  (bind _totaltime (Variables|/Game/Collab2024/Tech/IndividualWork/EvinOxley/BP_SpeedrunTimer.BP_SpeedrunTimer_C|GettotalTime _returnvalue))
  (if (>= (Variables|Default|GetRequired%20Number%20Left) (Utilities|Array|Length (stale EventTick _outactors)))
    (Default|Stop _returnvalue)
    (bind _returnvalue_2 (Class|GradeSystem|PlayerGrade (Variables|/Game/Collab2024/Tech/CoreItems/BP_GM_MainMode.BP_GM_MainMode_C|GetGradeSystem (Variables|Default|GetAs%20BP%20GM%20Main%20Mode)) (Math|Float|Truncate _totaltime)))
    (bind _asbp_game_instance (Utilities|Casting|CastToBP_GameInstance (Game|GetGameInstance)))
    (Class|GameInstanceSave|SaveLevelData _asbp_game_instance (Variables|/Game/Collab2024/Tech/IndividualWork/EvinOxley/BP_GameInstance.BP_GameInstance_C|GetIntLevelNum _asbp_game_instance) (Variables|/Game/Collab2024/Tech/IndividualWork/EvinOxley/BP_GameInstance.BP_GameInstance_C|GetInsRetries _asbp_game_instance) _totaltime _returnvalue_2)
    (Variables|/Game/Collab2024/Tech/IndividualWork/EvinOxley/BP_GameInstance.BP_GameInstance_C|SetInsRetries _asbp_game_instance 0)
    (bind _returnvalue_3 (UserInterface|CreateWidget "/Game/Collab2024/Tech/IndividualWork/TomLawrence/UI/Widgets/WBP_EndLevelScreen.WBP_EndLevelScreen_C"))
    (bind _output_get (Variables|Default|SetEndLevelScreen _returnvalue_3))
    (UserInterface|Viewport|AddtoViewport _output_get 0)
    (Rendering|Components|TextRender|SetText (Variables|/Game/Collab2024/Tech/IndividualWork/TomLawrence/UI/Widgets/WBP_EndLevelScreen.WBP_EndLevelScreen_C|GetText_Timer (Variables|Default|GetEndLevelScreen)) (Utilities|Text|ToText(Float) _totaltime "HalfToEven" false true 1 324 0 2))
    ;[1 1 1] Star Setting For Level Complete
    (switch int _returnvalue_2
      (:Default
        (Development|PrintString "INVALID"))
      (:0
        (Widget|SetVisibility (Variables|/Game/Collab2024/Tech/IndividualWork/TomLawrence/UI/Widgets/WBP_EndLevelScreen.WBP_EndLevelScreen_C|GetImage_Star0 (Variables|Default|GetEndLevelScreen)) "Visible"))
      (:1
        (Widget|SetVisibility (Variables|/Game/Collab2024/Tech/IndividualWork/TomLawrence/UI/Widgets/WBP_EndLevelScreen.WBP_EndLevelScreen_C|GetImage_Star1 (Variables|Default|GetEndLevelScreen)) "Visible"))
      (:2
        (Widget|SetVisibility (Variables|/Game/Collab2024/Tech/IndividualWork/TomLawrence/UI/Widgets/WBP_EndLevelScreen.WBP_EndLevelScreen_C|GetImage_Star2 (Variables|Default|GetEndLevelScreen)) "Visible"))
      (:3
        (Widget|SetVisibility (Variables|/Game/Collab2024/Tech/IndividualWork/TomLawrence/UI/Widgets/WBP_EndLevelScreen.WBP_EndLevelScreen_C|GetImage_Star3 (Variables|Default|GetEndLevelScreen)) "Visible")))))

(event EventTick
  (params (DeltaSeconds :type Float%20%28single-precision%29))
  (bind _outactors (Actor|GetAllActorsOfClass "/Game/Collab2024/Tech/IndividualWork/Jacob_Sirling/AI/BP_EnemyBase.BP_EnemyBase_C"))
  (Rendering|Components|TextRender|SetText (Variables|/Game/Collab2024/Tech/CoreItems/UI/WBP_HUD.WBP_HUD_C|GetEnemyCount (Variables|/Game/Collab2024/Tech/CoreItems/BP_GM_MainMode.BP_GM_MainMode_C|GetWBP_HUD (Variables|Default|GetAs%20BP%20GM%20Main%20Mode))) (Utilities|Text|FormatText "Enemies Left: {enemies}" (Utilities|Array|Length _outactors))))

(fn ConstructionScript)