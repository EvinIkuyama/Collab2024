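; Base class for player buff reactions, which spawn a colour-tinted Niagara pickup that expires unless the main character collects it in time.
; On overlap, it searches the player's BuffsAndDebuffs for a matching class, extending that buff's duration and destroying itself, or registering and activating itself.
; A delay loop consumes the duration, including extensions, before removal and delayed destruction.
; Empty BuffEvent and BuffEndEvent hooks leave the actual effect to child classes.
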(event Custom|OnBuffActivate
  (CallFunction|BuffEvent)
  ;[1 1 1] Check Buff Duration
  (Utilities|FlowControl|Delay (Variables|Default|GetDefault%20Duration) :!label _label)
  (bind _output_get (Variables|Default|SetEffect%20Duration (- (Variables|Default|GetEffect%20Duration) (Variables|Default|GetDefault%20Duration))))
  (if (> _output_get 0.0)
    (goto _label)
    (else
      (CallFunction|OnBuffEnd))))

(event Custom|OnBuffDurationExtend
  ;[1 0.8157 0.5167] Extend Buff Duration
  (bind _asbp_player_reaction_buff_base (Utilities|Casting|CastToBP_PlayerReactionBuffBase (Variables|Default|GetLocal%20Buff%20Reference)))
  (Variables|/Game/Collab2024/Tech/IndividualWork/JoeyLayton/Reactions/Reaction_Bases/BP_PlayerReactionBase.BP_PlayerReactionBase_C|SetEffect%20Duration _asbp_player_reaction_buff_base (+ (Variables|/Game/Collab2024/Tech/IndividualWork/JoeyLayton/Reactions/Reaction_Bases/BP_PlayerReactionBase.BP_PlayerReactionBase_C|GetEffect%20Duration _asbp_player_reaction_buff_base) (Variables|Default|GetEffect%20Duration)))
  (Actor|DestroyActor))

(event Custom|OnBuffEnd
  (CallFunction|BuffEndEvent)
  (Utilities|Array|RemoveItem (Variables|/Game/Collab2024/Tech/CoreItems/BP_MainCharacter.BP_MainCharacter_C|GetBuffs%20and%20Debuffs (Variables|Default|GetPlayer%20Editable)) self)
  (Utilities|FlowControl|Delay 5.0) ; Necessary but honestly annoying
  (Actor|DestroyActor))

(event Custom|BuffEvent)

(event Custom|BuffEndEvent)

(event Collision|EventActorBeginOverlap
  (params (OtherActor :type Actor%20Object%20Reference))
  (if (Class|GameplayStatics|ObjectIsA OtherActor "/Game/Collab2024/Tech/CoreItems/BP_MainCharacter.BP_MainCharacter_C")
    (Variables|Default|SetPlayer%20Picked%20Up true)
    ;[1 1 1] Remove in-world pickup
    (Components|DestroyComponent (Variables|Components|GetParticle%20Reference))
    ;;[1 1 1] Prevents Further Overlap
    (Components|DestroyComponent (Variables|Components|GetSphere))
    (CallFunction|SetPlayerRef OtherActor)
    (if (Utilities|Array|IsNotEmpty (Variables|/Game/Collab2024/Tech/CoreItems/BP_MainCharacter.BP_MainCharacter_C|GetBuffs%20and%20Debuffs (Variables|Default|GetPlayer%20Editable)))
      (bind _array_element (Utilities|Array|ForEachLoopwithBreak (Variables|/Game/Collab2024/Tech/CoreItems/BP_MainCharacter.BP_MainCharacter_C|GetBuffs%20and%20Debuffs (Variables|Default|GetPlayer%20Editable)) :!label _label)
        (:LoopBody
          (bind _return (CallFunction|CompareClass _array_element))
          (if _return
            (Variables|Default|SetLocal%20Buff%20Reference _array_element)
            (Variables|Default|SetReacting true)
            (goto _label Break)))
        (:Completed
          (if (Variables|Default|GetReacting) :!label _label_2
            (CallFunction|OnBuffDurationExtend)
            (else
              ;[1 1 1] Add Buff to Player
              (Utilities|Array|Add (Variables|/Game/Collab2024/Tech/CoreItems/BP_MainCharacter.BP_MainCharacter_C|GetBuffs%20and%20Debuffs (Variables|Default|GetPlayer%20Editable)) self)
              (CallFunction|OnBuffActivate)))))
      (else
        (goto _label_2)))))

(event EventOnReact
  (Variables|Default|SetDefault%20Duration (Variables|Default|GetEffect%20Duration))
  (bind _returnvalue (Niagara|SpawnSystematLocation "/Game/Collab2024/Tech/IndividualWork/JoeyLayton/NiagaraEffects/PS_Buff_Pickup.PS_Buff_Pickup" (Transformation|GetActorLocation))) ; Generic "Buff" pickup system
  (bind _output_get (Variables|Components|SetParticle%20Reference _returnvalue))
  (Niagara|SetNiagaraVariable(LinearColor) _output_get "Colour Minimum" (Variables|Default|GetBuff%20Pickup%20Colour%20One))
  (Niagara|SetNiagaraVariable(LinearColor) (Variables|Components|GetParticle%20Reference) "Colour Maximum" (Variables|Default|GetBuff%20Pickup%20Colour%20Two))
  (Utilities|FlowControl|Delay (Variables|Default|GetBuff%20PIckup%20Duration))
  (if (not (Variables|Default|GetPlayer%20Picked%20Up))
    (Components|Activation|Deactivate (Variables|Components|GetParticle%20Reference))
    (Actor|DestroyActor)))

(fn ConstructionScript)

(fn SetPlayerRef
  (params (Actor :type Actor%20Object%20Reference))
  (bind _asbp_main_character (Utilities|Casting|CastToBP_MainCharacter Actor))
  (Variables|Default|SetPlayer%20Editable _asbp_main_character)
  (return))

(fn CompareClass
  (params (Object :type Object%20Object%20Reference))
  (return (Class|GameplayStatics|ObjectIsA self (Utilities|GetClass Object))))